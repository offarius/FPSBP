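; BP_Muffin is an AI-controlled muffin character in MuffinWar that can attack other muffins and die.
; DoAttack turns on the hitbox, whose overlap instantly kills any other muffin; its switch-off branch is unreachable.
; Damage drains Health, and at zero prints a message, calls OnDeath and plays a falling sound.
; OnDeath runs once, disabling the hitbox and AI logic, then after a delay destroys the actor with pop sound and Niagara effect.
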(event `self.Hitbox.OnComponentBeginOverlap`
  (params (OverlappedComponent :type "PrimitiveComponent Object Reference") (OtherActor :type "Actor Object Reference") (OtherComp :type "PrimitiveComponent Object Reference") (OtherBodyIndex :type Integer) (bFromSweep :type Boolean) (SweepResult :type "HitResult Structure (by ref)"))
  (bind _asbp_muffin (cast `/Game/MuffinWar/Characters/Muffin/Blueprints/BP_Muffin` OtherActor))
  (`self.OnDeath` _asbp_muffin))

(event `OnDeath`
  (if (not (`self.IsDead`))
    (`PrimitiveComponent.SetCollisionEnabled` (`self.Hitbox`) "NoCollision")
    (set `self.IsDead` true)
    (`BrainComponent.StopLogic` (`AIController.BrainComponent` (`AIBlueprintHelperLibrary.GetAIController` self)) "")
    (`KismetSystemLibrary.Delay` 1.5)
    (`self.K2_DestroyActor`)
    (`GameplayStatics.PlaySoundAtLocation` "/Game/Audio/Interface_And_Item_Sounds/Cues/Abstract_Pop_03_Cue.Abstract_Pop_03_Cue" (0.0 0.0 0.0) (struct) 1.0 1.0 0.0 null null null null)
    (`AddComponent|NODE_AddNiagaraComponent-1`)))

(event `self.ReceiveAnyDamage`
  (params (Damage :type "Float (single-precision)") (DamageType :type "DamageType Object Reference") (InstigatedBy :type "Controller Object Reference") (DamageCauser :type "Actor Object Reference"))
  (bind _output_get (set `self.Health` (- (`self.Health`) Damage)))
  (if (<= _output_get 0.0)
    (`KismetSystemLibrary.PrintString` "SCAV RUN!" true true (struct :`R` 1.0 :`B` 0.024992 :`A` 1.0))
    (`self.OnDeath`)
    (`GameplayStatics.PlaySoundAtLocation` "/Game/Audio/Interface_And_Item_Sounds/Cues/Cartoon_Falling_05_Cue.Cartoon_Falling_05_Cue" (0.0 0.0 0.0) (struct) 1.0 1.0 0.0 null null null null)
    (`KismetSystemLibrary.Delay` 1.5)))

(fn `DoAttack`
  (params (IsAttacking :type Boolean))
  (if true
    (`PrimitiveComponent.SetCollisionEnabled` (`self.Hitbox`) "QueryOnly")))

(fn `UserConstructionScript`)