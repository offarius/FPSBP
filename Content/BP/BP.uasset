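; Trigger-box Blueprint that rescales one static mesh and swaps another's material when something enters or leaves the box.
; Begin and end overlap each play their own timeline, whose three tracks set StaticMesh1's world scale at its current location, with rotation left at default.
; Those updates also set StaticMesh2 to BasicAsset03 on entry and ArrowMaterial on exit.
; Timelines use Play rather than PlayFromStart, and overlaps are unfiltered.
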(event `self.Box.OnComponentBeginOverlap`
  (params (OverlappedComponent :type "PrimitiveComponent Object Reference") (OtherActor :type "Actor Object Reference") (OtherComp :type "PrimitiveComponent Object Reference") (OtherBodyIndex :type Integer) (bFromSweep :type Boolean) (SweepResult :type "HitResult Structure (by ref)"))
  (bind (_direction _newtrack_0 _newtrack_1 _newtrack_2) (`Timeline|Timeline`)
    (:`Update`
      (`SceneComponent.K2_SetWorldTransform` (`self.StaticMesh1`) (`KismetMathLibrary.MakeTransform` (`SceneComponent.K2_GetComponentLocation` (`self.StaticMesh1`)) (struct) (`KismetMathLibrary.MakeVector` _newtrack_0 _newtrack_1 _newtrack_2)) false false)
      (`PrimitiveComponent.SetMaterial` (`self.StaticMesh2`) 0 "/Engine/MapTemplates/Materials/BasicAsset03.BasicAsset03"))))

(event `self.Box.OnComponentEndOverlap`
  (params (OverlappedComponent :type "PrimitiveComponent Object Reference") (OtherActor :type "Actor Object Reference") (OtherComp :type "PrimitiveComponent Object Reference") (OtherBodyIndex :type Integer))
  (bind (_direction _newtrack_0 _newtrack_1 _newtrack_2) (`Timeline|Timeline_0`)
    (:`Update`
      (`SceneComponent.K2_SetWorldTransform` (`self.StaticMesh1`) (`KismetMathLibrary.MakeTransform` (`SceneComponent.K2_GetComponentLocation` (`self.StaticMesh1`)) (struct) (`KismetMathLibrary.MakeVector` _newtrack_0 _newtrack_1 _newtrack_2)) false false)
      (`PrimitiveComponent.SetMaterial` (`self.StaticMesh2`) 0 "/Engine/VREditor/UI/ArrowMaterial.ArrowMaterial"))))

(fn `UserConstructionScript`)