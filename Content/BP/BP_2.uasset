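; BP_2 is an actor Blueprint that appears to be a sandbox for flow-control nodes, with debug prints.
; BeginPlay switches on KAWOEnum to print the state number.
; Static mesh hits alternate via FlipFlop between calling TurnMessage and OffMessage on a referenced actor.
; A placeholder-named function and macro, unused here, hold index-printing loops that exit from the loop body, and the macro adds a second exec path with a green print.
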(event `self.ReceiveBeginPlay`
  (switch `/Game/BP/Data/KAWO_Enum` (`self.KAWO_Enum`)
    (:`NewEnumerator0`
      (`KismetSystemLibrary.PrintString` "1"))
    (:`NewEnumerator1`
      (`KismetSystemLibrary.PrintString` "2"))
    (:`NewEnumerator2`
      (`KismetSystemLibrary.PrintString` "3"))
    (:`NewEnumerator3`
      (`KismetSystemLibrary.PrintString` "4"))))

(event `self.StaticMesh.OnComponentHit`
  (params (HitComponent :type "PrimitiveComponent Object Reference") (OtherActor :type "Actor Object Reference") (OtherComp :type "PrimitiveComponent Object Reference") (NormalImpulse :type "Vector Structure") (Hit :type "HitResult Structure (by ref)"))
  (bind _actor_ref (`self.actor_ref`))
  (`/Engine/EditorBlueprintResources/StandardMacros.FlipFlop`
    (:`A`
      (message `/Game/BP/STYL.turn` _actor_ref))
    (:`B`
      (message `/Game/BP/STYL.off` _actor_ref))))

(fn `NewFunction`
  (params (NewParam3 :type Boolean) (NewParam4 :type Boolean) (NewParam5 :type Boolean))
  (returns (NewParam :type Boolean) (NewParam1 :type Boolean) (NewParam2 :type Boolean))
  (for _index (range (`self.NewVar`) 1)
    (`KismetSystemLibrary.PrintString` (`KismetStringLibrary.Conv_IntToString` _index))
    (return false false false)))

(fn `UserConstructionScript`)